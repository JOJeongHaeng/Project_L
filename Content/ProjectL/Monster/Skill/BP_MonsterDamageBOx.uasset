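; BP_MonsterDamageBOx is a short-lived hit box for boss monster skills that damages actors tagged Player when they overlap it.
; On BeginPlay it scales its collision box and sets a one-second lifespan.
; Both box scale and damage come from DT_BossSkill, found by looping all rows for the one whose AnimMontage matches the box's DamageMontage variable.
; Debug strings print the applied damage and missing rows.
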(event `self.ReceiveBeginPlay`
  (`self.DamageSize`)
  (`self.SetLifeSpan` 1.0))

(event `self.ReceiveActorBeginOverlap`
  (params (OtherActor :type "Actor Object Reference"))
  (if (`self.ActorHasTag` OtherActor "Player")
    (`self.ApplyDamage` OtherActor)))

(fn `ApplyDamage`
  (params (DamagedActor :type "Actor Object Reference"))
  (locals (DamageAnimSequ :type "AnimSequenceBase Object Reference") (Actor :type "Actor Object Reference"))
  (set `local.Actor` DamagedActor)
  (bind _outrownames (`DataTableFunctionLibrary.GetDataTableRowNames` "/Game/ProjectL/Monster/Skill/DT_BossSkill.DT_BossSkill"))
  (for _array_element _outrownames
    (bind _returnvalue (`|GetDataTableRow` "/Game/ProjectL/Monster/Skill/DT_BossSkill.DT_BossSkill" _array_element)
      (:`then`
        (bind (_name _animmontage _cooltime _damage) (break `/Game/ProjectL/Monster/Skill/ST_BossSkill` _returnvalue))
        (if (== (`self.DamageMontage`) _animmontage)
          (bind _returnvalue_2 (`GameplayStatics.ApplyDamage` (`local.Actor`) _damage))
          (`KismetSystemLibrary.PrintString` (`KismetStringLibrary.Concat_StrStr` "Apply Damage : " (`KismetStringLibrary.Conv_DoubleToString` _returnvalue_2)) true true (struct :`R` 1.0 :`G` 0.016606 :`A` 1.0))))
      (:`RowNotFound`
        (`KismetSystemLibrary.PrintString` "DamageBoxBindedevent RownotFound")))))

(fn `DamageSize`
  (bind _outrownames (`DataTableFunctionLibrary.GetDataTableRowNames` "/Game/ProjectL/Monster/Skill/DT_BossSkill.DT_BossSkill"))
  (for _array_element _outrownames
    (bind _returnvalue (`|GetDataTableRow` "/Game/ProjectL/Monster/Skill/DT_BossSkill.DT_BossSkill" _array_element)
      (:`then`
        (bind (_name _animmontage _cooltime _damage _damagesize) (break `/Game/ProjectL/Monster/Skill/ST_BossSkill` _returnvalue))
        (if (== (`self.DamageMontage`) _animmontage)
          (`SceneComponent.SetWorldScale3D` (`self.DamageBox_Clollision`) _damagesize)))
      (:`RowNotFound`
        (`KismetSystemLibrary.PrintString` "DamageBox Size RownotFound")))))

(fn `UserConstructionScript`)