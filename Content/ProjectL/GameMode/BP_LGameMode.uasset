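; BP_LGameMode is a game mode that launches the level's gimmick hazards once the Gimmic flag is set.
; Tick polls that flag and, after a short Delay, calls the IsGimmic dispatcher, spawns the balls and bar, then sets GimmicPlay to prevent repeats.
; A looping timer runs SpawnFloor, which spawns a floor actor at one of two random scales.
; An unconnected copy of the spawn sequence never runs.
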(event `self.ReceiveBeginPlay`)

(event `self.ReceiveTick`
  (params (DeltaSeconds :type "Float (single-precision)"))
  (bind _gimmic (`self.Gimmic`))
  (if (`self.GimmicPlay`)
    _
    (elif _gimmic
      (`KismetSystemLibrary.Delay` 5.0)
      (`self.EventDispatcher_IsGimmic` _gimmic)
      (`self.SpawnGimmicBall`)
      (`|SpawnActorFromClass` "/Game/ProjectL/GameMode/Gimmicmap/BP_GimmicBar.BP_GimmicBar_C" (`KismetMathLibrary.MakeTransform` (0.0 0.0 10.0)) "Undefined" "MultiplyWithRoot" null null)
      (`KismetSystemLibrary.K2_SetTimer` null "SpawnFloor" 3.5 true)
      (set `self.GimmicPlay` true))))

(fn `SpawnFloor`
  (if (`KismetMathLibrary.RandomBool`)
    (`|SpawnActorFromClass` "/Game/ProjectL/GameMode/Gimmicmap/BP_GimmicFloor.BP_GimmicFloor_C" (`KismetMathLibrary.MakeTransform` (0.0 0.0 10.0) (struct) (30.0 30.0 1.0)) "Undefined" "MultiplyWithRoot" null null)
    (else
      (`|SpawnActorFromClass` "/Game/ProjectL/GameMode/Gimmicmap/BP_GimmicFloor.BP_GimmicFloor_C" (`KismetMathLibrary.MakeTransform` (0.0 0.0 10.0) (struct) (42.0 42.0 1.0)) "Undefined" "MultiplyWithRoot" null null))))

(fn `SpawnGimmicBall`
  (`|SpawnActorFromClass` "/Game/ProjectL/GameMode/Gimmicmap/BP_GimmicBalls.BP_GimmicBalls_C" (`KismetMathLibrary.MakeTransform` (0.0 0.0 0.0)) "Undefined" "MultiplyWithRoot" null null))

(fn `UserConstructionScript`)