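; BP_PlayerState holds a player's Identity counter and runs a timed stun that locks movement.
; On BeginPlay it binds to the player controller's identity update event; UpdateIdentity adds the change, clamps the counter and prints it.
; While ISStun is set, Tick spawns BP_Stun once at the pawn's XY at a fixed height.
; It holds the controller's CanMove false for about a second, then resets.
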(event `self.ReceiveBeginPlay`
  (bind _asbp_player_controller (cast `/Game/ProjectL/GameMode/Player/BP_PlayerController` (`GameplayStatics.GetPlayerController` 0)))
  (add `/Game/ProjectL/GameMode/Player/BP_PlayerController.UpdateIdentity` _asbp_player_controller (`|CreateDelegate` :!event `UpdateIdentity`)))

(event `self.ReceiveTick`
  (params (DeltaSeconds :type "Float (single-precision)"))
  (`self.Stun ` DeltaSeconds))

(fn `Stun `
  (params (B :type "Float (double-precision)"))
  (if (`self.ISStun`)
    (set `self.StunTime` (+ (`self.StunTime`) B))
    (if (not (`self.StunActorSpawned`))
      ; 고칠부분(완료)
      (bind _asbp_lgame_pawn (cast `/Game/ProjectL/GameMode/Player/Character/BP_LGamePawn` (`Controller.K2_GetPawn` (`GameplayStatics.GetPlayerController` 0))))
      (bind _returnvalue (`self.GetTransform` _asbp_lgame_pawn))
      (`|SpawnActorFromClass` "/Game/ProjectL/GameMode/Player/Character/PlayerState/BP_Stun.BP_Stun_C" (`KismetMathLibrary.MakeTransform` (`KismetMathLibrary.MakeVector` (.x (.location _returnvalue)) (.y (.location _returnvalue)) 200.0) (.rotation _returnvalue)) "Undefined" "MultiplyWithRoot" null null)
      (set `self.StunActorSpawned` true))
    (if (> (`self.StunTime`) 1.0)
      (set `self.StunTime` 0.0)
      (bind _asbp_player_controller (cast `/Game/ProjectL/GameMode/Player/BP_PlayerController` (`GameplayStatics.GetPlayerController` 0))
        (:`then`
          (set `/Game/ProjectL/GameMode/Player/BP_PlayerController.CanMove` true _asbp_player_controller)
          (set `self.ISStun` false)
          (set `self.StunActorSpawned` false))
        (:`CastFailed`
          (`KismetSystemLibrary.PrintString` "cast failed")))
      (else
        (bind _asbp_player_controller_2 (cast `/Game/ProjectL/GameMode/Player/BP_PlayerController` (`GameplayStatics.GetPlayerController` 0))
          (:`then`
            (set `/Game/ProjectL/GameMode/Player/BP_PlayerController.CanMove` false _asbp_player_controller_2))
          (:`CastFailed`
            (`KismetSystemLibrary.PrintString` "cast failed")))))))

(fn `UpdateIdentity`
  (params (updateCount :type Integer))
  (bind _output_get (set `self.Identity` (`KismetMathLibrary.Clamp` (+ updateCount (`self.Identity`)) 0 2)))
  (`KismetSystemLibrary.PrintString` (`KismetStringLibrary.Concat_StrStr` "Identity is" (`KismetStringLibrary.Conv_IntToString` _output_get))))

(fn `UserConstructionScript`)