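; BP_Stun is a short-lived stun effect actor that orbits a static mesh above the first player's pawn and destroys itself after a fixed lifespan.
; Each tick it accumulates time and, while the pawn's BP_PlayerState reports ISStun, uses sine and cosine to circle the mesh around the pawn's mesh.
; It always follows player controller 0's pawn and prints a debug message when either cast fails.
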(event `self.ReceiveBeginPlay`
  (`self.SetLifeSpan` 2.0))

(event `self.ReceiveTick`
  (params (DeltaSeconds :type "Float (single-precision)"))
  (bind _radius (`self.Radius`))
  (bind _returnvalue (* (`self.time`) 180.0))
  (set `self.time` (+ DeltaSeconds (`self.time`)))
  (bind _asbp_lgame_pawn (cast `/Game/ProjectL/GameMode/Player/Character/BP_LGamePawn` (`Controller.K2_GetPawn` (`GameplayStatics.GetPlayerController` 0)))
    (:`then`
      (bind _asbp_player_state (cast `/Game/ProjectL/GameMode/Player/BP_PlayerState` (`Pawn.PlayerState` _asbp_lgame_pawn))
        (:`then`
          (if (`/Game/ProjectL/GameMode/Player/BP_PlayerState.ISStun` _asbp_player_state)
            (`SceneComponent.K2_SetWorldLocation` (`self.StaticMesh`) (+ (`KismetMathLibrary.MakeVector` (* _radius (`KismetMathLibrary.Sin` (`KismetMathLibrary.DegreesToRadians` _returnvalue))) (* (`KismetMathLibrary.Cos` (`KismetMathLibrary.DegreesToRadians` _returnvalue)) _radius) 200.0) (`SceneComponent.K2_GetComponentLocation` (`Character.Mesh` _asbp_lgame_pawn))) false false)))
        (:`CastFailed`
          (`KismetSystemLibrary.PrintString` "BPstun Castfailed2"))))
    (:`CastFailed`
      (`KismetSystemLibrary.PrintString` "BPstun Castfailed"))))

(fn `UserConstructionScript`)