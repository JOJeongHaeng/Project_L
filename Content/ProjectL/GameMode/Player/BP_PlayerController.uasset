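; Player controller for a mouse-driven game that moves its BP_LGamePawn by right-click click-to-move.
; Init shows the cursor, enables click events and binds an ApplyDamage event.
; Right-click traces under the cursor, draws a debug sphere and calls SimpleMoveToLocation while CanMove is true; Tick halts movement otherwise.
; Helper functions spawn a DamageBox ahead of the pawn carrying its current montage, and check whether PlayerState Identity is above zero.
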(event `self.ReceiveBeginPlay`
  ; mouse 보이게 + click event
  (`self.Init`))

(event `EnhancedInput|/Game/ProjectL/GameMode/Player/InputAction/IA_RightMouse`
  (params (ActionValue :type Boolean) (ElapsedSeconds :type "Float (double-precision)") (TriggeredSeconds :type "Float (double-precision)") (InputAction :type "InputAction Object Reference" :default "/Game/ProjectL/GameMode/Player/InputAction/IA_RightMouse.IA_RightMouse"))
  ; 마우스 input 으로 움직임 구현
  (:`Started`
    (`self.MouseClickMoveMent` :!label _label))
  (:`Ongoing`
    (goto _label)))

(event `self.ReceiveTick`
  (params (DeltaSeconds :type "Float (single-precision)"))
  (if (not (`self.CanMove`))
    (`self.StopMovement`)))

(fn `CanUseIdentity`
  (returns (CanUse :type Boolean))
  (bind _asbp_player_state (cast `/Game/ProjectL/GameMode/Player/BP_PlayerState` (`self.PlayerState`))
    (:`then`
      (if (<= (`/Game/ProjectL/GameMode/Player/BP_PlayerState.Identity` _asbp_player_state) 0)
        (return false)
        (else
          (return true))))
    (:`CastFailed`
      (`KismetSystemLibrary.PrintString` "Controller to StateCastFailed"))))

(fn `Init`
  (set `self.bShowMouseCursor` true)
  (set `self.bEnableClickEvents` true)
  (set `self.bEnableMouseOverEvents` true)
  ; bind
  (add `self.ApplyDamage` (`|CreateDelegate` :!event `SpawnDamageBox`)))

(fn `MouseClickMoveMent`
  (bind (_bblockinghit _binitialoverlap _time _distance _location) (`GameplayStatics.BreakHitResult` (`self.GetHitResultUnderCursorByChannel` "TraceTypeQuery1")))
  (if (`self.CanMove`)
    (cast `/Game/ProjectL/GameMode/Player/Character/BP_LGamePawn` (`self.K2_GetPawn`))
    (`KismetSystemLibrary.DrawDebugSphere` _location 100.0 12 (struct :`R` 1.0 :`G` 0.02448 :`A` 1.0) 5.0)
    (`AIBlueprintHelperLibrary.SimpleMoveToLocation` self _location)))

(fn `SpawnDamageBox`
  (params (Animation :type "AnimSequenceBase Object Reference"))
  (bind _returnvalue (`self.K2_GetPawn`))
  (bind _returnvalue_2 (`self.GetActorForwardVector` _returnvalue))
  (bind (_returnvalue_roll _returnvalue_pitch _returnvalue_yaw) (`KismetMathLibrary.BreakRotator` (`KismetMathLibrary.MakeRotFromX` _returnvalue_2)))
  (bind _asbp_lgame_pawn (cast `/Game/ProjectL/GameMode/Player/Character/BP_LGamePawn` _returnvalue))
  (`|SpawnActorFromClass` "/Game/ProjectL/GameMode/Player/Skill/Damage/DamageBox.DamageBox_C" (`KismetMathLibrary.MakeTransform` (+ (`self.K2_GetActorLocation` _returnvalue) (* _returnvalue_2 270.0)) (`KismetMathLibrary.MakeRotator` _returnvalue_roll _returnvalue_pitch (+ _returnvalue_yaw 90.0))) "Undefined" "MultiplyWithRoot" null (`Character.GetCurrentMontage` _asbp_lgame_pawn) null))

(fn `UserConstructionScript`)