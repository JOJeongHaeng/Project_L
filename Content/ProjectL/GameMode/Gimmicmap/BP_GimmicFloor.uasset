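; BP_GimmicFloor is a short-lived floor hazard actor that stuns and damages overlapping player pawns.
; One second after BeginPlay it enables query-and-physics collision on its seven static meshes, then destroys itself 0.1 seconds later, giving a delayed, momentary hit window.
; On actor overlap it casts to BP_LGamePawn and its BP_PlayerState, sets the stun flag and applies heavy damage, with debug prints for success and failed casts.
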(event `self.ReceiveBeginPlay`
  (`KismetSystemLibrary.Delay` 1.0)
  (`PrimitiveComponent.SetCollisionEnabled` (`self.StaticMesh`) "QueryAndPhysics")
  (`PrimitiveComponent.SetCollisionEnabled` (`self.StaticMesh3`) "QueryAndPhysics")
  (`PrimitiveComponent.SetCollisionEnabled` (`self.StaticMesh4`) "QueryAndPhysics")
  (`PrimitiveComponent.SetCollisionEnabled` (`self.StaticMesh1`) "QueryAndPhysics")
  (`PrimitiveComponent.SetCollisionEnabled` (`self.StaticMesh2`) "QueryAndPhysics")
  (`PrimitiveComponent.SetCollisionEnabled` (`self.StaticMesh5`) "QueryAndPhysics")
  (`PrimitiveComponent.SetCollisionEnabled` (`self.StaticMesh6`) "QueryAndPhysics")
  (`KismetSystemLibrary.Delay` 0.1)
  (`self.K2_DestroyActor`))

(event `self.ReceiveActorBeginOverlap`
  (params (OtherActor :type "Actor Object Reference"))
  (`KismetSystemLibrary.PrintString` "overlap Success")
  (bind _asbp_lgame_pawn (cast `/Game/ProjectL/GameMode/Player/Character/BP_LGamePawn` OtherActor)
    (:`then`
      (bind _asbp_player_state (cast `/Game/ProjectL/GameMode/Player/BP_PlayerState` (`Pawn.PlayerState` _asbp_lgame_pawn))
        (:`then`
          (set `/Game/ProjectL/GameMode/Player/BP_PlayerState.ISStun` true _asbp_player_state)
          (`KismetSystemLibrary.PrintString` "Stun!")
          (`GameplayStatics.ApplyDamage` _asbp_lgame_pawn 1000.0))
        (:`CastFailed`
          (`KismetSystemLibrary.PrintString` "Floor cast failed2"))))
    (:`CastFailed`
      (`KismetSystemLibrary.PrintString` "Floor cast failed"))))

(fn `UserConstructionScript`)